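; Balloon actor that can be picked up, dropped off and popped by a button popper.
; BeginPlay binds Popped to the PopBalloons dispatcher on the first Bp_buttonpopper found in the level.
; PickUp disables mesh physics and attaches the root to the given component, while DropOff restores physics, detaches and adds an upward impulse.
; Popped plays a pop sound, spawns confetti and destroys the balloon.
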(event `self.ReceiveBeginPlay`
  (bind _outactors (`GameplayStatics.GetAllActorsOfClass` "/Game/Assets/blueprints/bp_buttonpopper.bp_buttonpopper_C"))
  (bind _output_get (set `self.buttons` (`KismetArrayLibrary.Array_Get` _outactors)))
  (add `/Game/Assets/blueprints/bp_buttonpopper.popBalloons` _output_get (delegate `Popped`)))

(event `/Game/Assets/blueprints/PickUpInterface.PickUp`
  (params (ActorToAttachTo :type "SceneComponent Object Reference"))
  (`PrimitiveComponent.SetSimulatePhysics` (`self.balloon_mesh`) false)
  (`SceneComponent.K2_AttachToComponent` (`self.K2_GetRootComponent`) ActorToAttachTo "None" "KeepWorld" "KeepWorld" "KeepWorld" true))

(event `Popped`
  (`GameplayStatics.PlaySoundAtLocation` "/Game/Assets/audio/a_balloonPop_Cue.a_balloonPop_Cue" (`SceneComponent.K2_GetComponentLocation` (`self.balloon_mesh`)))
  (`GameplayStatics.SpawnEmitterAtLocation` "/Game/Assets/particles/p_confetti.p_confetti" (`self.K2_GetActorLocation`))
  (`self.K2_DestroyActor`))

(event `/Game/Assets/blueprints/PickUpInterface.dropOff`
  (`PrimitiveComponent.SetSimulatePhysics` (`self.balloon_mesh`) true)
  (`self.K2_DetachFromActor` "KeepWorld" "KeepWorld" "KeepWorld")
  (`PrimitiveComponent.AddImpulse` (`self.balloon_mesh`) (0.0 0.0 50.0) "None" false))

(fn `UserConstructionScript`)